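; CustomPlayerController is a player controller that sets up the local HUD and provides a debug score readout.
; On BeginPlay, the local controller creates the HeadsUpDisplay widget, stores it and adds it to the viewport.
; Pressing Tab loops over the GameState PlayerArray, casts each entry to CustomPlayerState and prints its player ID with its GoalA and GoalB points.
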(event EventTick
  (params (DeltaSeconds :type Float%20%28single-precision%29)))

(event EventBeginPlay
  (Utilities|FlowControl|Sequence
    (:then_0
      (if (Pawn|IsLocalPlayerController)
        (bind _returnvalue (UserInterface|CreateWidget "/Game/Rocket/HeadsUpDisplay.HeadsUpDisplay_C"))
        (bind _output_get (Variables|Default|SetHeadsUpDisplay _returnvalue))
        (UserInterface|Viewport|AddtoViewport _output_get 0)))))

(event Input|KeyboardEvents|Tab
  (params (Key :type Key%20Structure :default "None"))
  (:Pressed
    (for _array_element (Variables|/Script/Engine.GameStateBase|GetPlayerArray (Game|GetGameState))
      (bind _ascustom_player_state (Utilities|Casting|CastToCustomPlayerState _array_element))
      (Development|PrintString (Utilities|String|ToString(Text) (Utilities|Text|FormatText "Player ID: {id}     GoalA:  {score A}      GoalB: {score B}" (Variables|/Script/Engine.PlayerState|GetPlayerId _ascustom_player_state) (Variables|/Game/Rocket/CustomPlayerState.CustomPlayerState_C|GetPointsGoalA _ascustom_player_state) (Variables|/Game/Rocket/CustomPlayerState.CustomPlayerState_C|GetPointsGoalB _ascustom_player_state)))))))

(fn ConstructionScript)